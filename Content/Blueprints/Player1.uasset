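; Player 1 pawn for a timed Bomberman-style game, moving a cube by force and dropping bombs with Space Bar.
; Tick turns the Player 1 movement axes into acceleration until the GameInstance flags time up, then stops applying force and resets speed and bomb limit.
; Longer-blast and speed-up pickup flags each start a ten-second timer that restores defaults, using resettable DoOnce gates.
; Bombs spawn at the cube's position, raised in Z, until the count reaches its maximum.
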(event EventBeginPlay
  (bind _asgame_instance_bomb (Utilities|Casting|CastToGameInstance_Bomb (Game|GetGameInstance)))
  (Variables|Default|SetGameInstance _asgame_instance_bomb))

(event Collision|EventActorBeginOverlap
  (params (OtherActor :type Actor%20Object%20Reference)))

(event EventTick
  (params (DeltaSeconds :type Float%20%28single-precision%29))
  (if (Variables|/Game/Blueprints/GameInstance_Bomb.GameInstance_Bomb_C|GetTimesUp (Variables|Default|GetGameInstance))
    (Utilities|FlowControl|DoOnce false
      (:Completed
        (Variables|Default|SetMovementSpeed 1e+04)
        (Variables|Default|SetMaxBombNumber 1)))
    (else
      (Physics|AddForce (Variables|Default|GetPlayer1Cube) (Math|Vector|MakeVector (* (Input|AxisValues|GetMoveForward1) (Variables|Default|GetMovementSpeed)) (* (Input|AxisValues|GetMoveRight1) (Variables|Default|GetMovementSpeed)) 0.0) "None" true)
      (Utilities|FlowControl|Sequence
        (:then_0
          ;[1 1 1] Reset LangerBlaster and SpeedUp pickup
          (if (Variables|Default|GetbHasLongerBlaster)
            (Utilities|FlowControl|DoOnce false :!label _label
              (:Completed
                (Utilities|FlowControl|Delay 1e+01)
                (Variables|/Game/Blueprints/GameInstance_Bomb.GameInstance_Bomb_C|SetBox1Size (Variables|Default|GetGameInstance) "55.000000,300.000000,100.000000")
                (Variables|Default|SetbHasLongerBlaster false)
                (goto _label Reset)))))
        (:then_1
          (if (Variables|Default|GetbHasSpeedUp)
            (Utilities|FlowControl|DoOnce false :!label _label_2
              (:Completed
                (Utilities|FlowControl|Delay 1e+01)
                (Variables|Default|SetMovementSpeed 1e+04)
                (Variables|Default|SetbHasSpeedUp false)
                (goto _label_2 Reset)))))))))

(event Input|KeyboardEvents|SpaceBar
  (params (Key :type Key%20Structure))
  (bind _player1cube (Variables|Default|GetPlayer1Cube))
  (bind _returnvalue (Transformation|GetWorldLocation _player1cube))
  (bind (_x _y _z) (Math|Vector|BreakVector _returnvalue))
  ;[1 1 1] Press Space Bar to place a BOMB!
  (:Pressed
    (if (!= (Variables|Default|GetBombs) (Variables|Default|GetMaxBombNumber))
      (Game|SpawnActorfromClass "/Game/Blueprints/Bomb.Bomb_C" (Math|Conversions|ToTransform(Vector) (Math|Vector|MakeVector _x _y (- _z -1.5e+02))) "Undefined" 0 0)
      (Math|Integer|IncrementInt (Variables|Default|GetBombs)))))

(fn ConstructionScript)