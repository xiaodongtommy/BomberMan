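; BreakWall is a breakable wall that may drop a power-up pickup when destroyed.
; Its Destroyed event calls OddToDrop, which spawns either an extra-bomb, longer-blast or player-speedup pickup at the BreakableWall component's location, or nothing.
; Selection is a cascade of percentage checks, each with its own random roll, so the drop odds are not equal quarters.
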(event EventBeginPlay)

(event Collision|EventActorBeginOverlap
  (params (OtherActor :type Actor%20Object%20Reference)))

(event EventTick
  (params (DeltaSeconds :type Float%20%28single-precision%29)))

(event EventDestroyed
  (CallFunction|OddtoDrop))

(fn ConstructionScript)

(fn OddtoDrop
  (bind _returnvalue (Math|Random|RandomFloatinRange 0.0 1e+02))
  (bind _breakablewall (Variables|Default|GetBreakableWall))
  (bind _returnvalue_2 (Transformation|GetWorldLocation _breakablewall))
  (if (<= _returnvalue 25.0)
    (Game|SpawnActorfromClass "/Game/Blueprints/PK_MoreBomb.PK_MoreBomb_C" (Math|Conversions|ToTransform(Vector) (Transformation|GetWorldLocation (Variables|Default|GetBreakableWall))) "Undefined" 0 0)
    (elif (>= _returnvalue 75.0)
      (Game|SpawnActorfromClass "/Game/Blueprints/PK_LongerBombBlaste.PK_LongerBombBlaste_C" (Math|Conversions|ToTransform(Vector) _returnvalue_2) "Undefined" 0 0)
      (elif (and (>= _returnvalue 26.0) (<= _returnvalue 5e+01))
        (Game|SpawnActorfromClass "/Game/Blueprints/PK_PlayerSpeedup.PK_PlayerSpeedup_C" (Math|Conversions|ToTransform(Vector) _returnvalue_2) "Undefined" 0 0)))))