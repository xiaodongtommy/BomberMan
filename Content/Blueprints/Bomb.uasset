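; Bomberman-style bomb actor that explodes three seconds after BeginPlay.
; On detonation it decrements the Bombs counter on every Player1 actor, with no equivalent step for Player2.
; It then queries two box components, Box and Box1, destroying any overlapping Player1, Player2 or BreakWall actors, and finally destroys itself.
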(event EventBeginPlay
  (Utilities|FlowControl|Delay 3.0)
  (bind _outactors (Actor|GetAllActorsOfClass "/Game/Blueprints/Player1.Player1_C"))
  (for _array_element _outactors
    (Math|Integer|DecrementInt (Variables|/Game/Blueprints/Player1.Player1_C|GetBombs _array_element)))
  (Utilities|FlowControl|Sequence
    (:then_0
      (bind _output_get (Variables|Default|SetObjectsOverlapping (Collision|GetOverlappingActors (Variables|Default|GetBox) 0 :!class /Script/Engine.PrimitiveComponent)))
      (for _array_element_2 _output_get
        (if (or (== (Utilities|GetClass _array_element_2) "/Game/Blueprints/Player1.Player1_C") (== (Utilities|GetClass _array_element_2) "/Game/Blueprints/Player2.Player2_C"))
          (Actor|DestroyActor _array_element_2)
          (elif (== (Utilities|GetClass _array_element_2) "/Game/Blueprints/BreakWall.BreakWall_C")
            (bind _asbreak_wall (Utilities|Casting|CastToBreakWall _array_element_2))
            (Actor|DestroyActor _asbreak_wall)))))
    (:then_1
      (bind _output_get_2 (Variables|Default|SetObjectsOverlapping2 (Collision|GetOverlappingActors (Variables|Default|GetBox1) 0 :!class /Script/Engine.PrimitiveComponent)))
      (for _array_element_3 _output_get_2
        (if (or (== (Utilities|GetClass _array_element_3) "/Game/Blueprints/Player1.Player1_C") (== (Utilities|GetClass _array_element_3) "/Game/Blueprints/Player2.Player2_C"))
          (Actor|DestroyActor _array_element_3)
          (elif (== (Utilities|GetClass _array_element_3) "/Game/Blueprints/BreakWall.BreakWall_C")
            (bind _asbreak_wall_2 (Utilities|Casting|CastToBreakWall _array_element_3))
            (Actor|DestroyActor _asbreak_wall_2))))
      (Actor|DestroyActor))))

(event Collision|EventActorBeginOverlap
  (params (OtherActor :type Actor%20Object%20Reference)))

(event EventTick
  (params (DeltaSeconds :type Float%20%28single-precision%29)))

(fn ConstructionScript)