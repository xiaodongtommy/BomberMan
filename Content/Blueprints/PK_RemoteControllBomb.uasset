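; Pickup actor that turns a player's bomb into a remote-controlled bomb, usable by Player1 or Player2.
; On box overlap it checks the player class, stores a fixed box size for that player in GameInstance_Bomb, and sets the bomb to BombRemote.
; It also copies MaxBombNumber into MaxBombTemp and flags HasRemoteBomb, then destroys itself.
; Each player has a duplicate branch writing its own variables.
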(event OnComponentBeginOverlap(Box)
  (params (OverlappedComponent :type Primitive%20Component%20Object%20Reference) (OtherActor :type Actor%20Object%20Reference) (OtherComp :type Primitive%20Component%20Object%20Reference) (OtherBodyIndex :type Integer) (bFromSweep :type Boolean) (SweepResult :type Hit%20Result%20Structure%20%28by%20ref%29))
  (bind _returnvalue (Utilities|GetClass OtherActor))
  (bind _returnvalue_2 (Game|GetGameInstance))
  (if (== _returnvalue "/Game/Blueprints/Player1.Player1_C")
    ;[1 1 1] Make bomb a remote bomb.
    (bind _asgame_instance_bomb (Utilities|Casting|CastToGameInstance_Bomb _returnvalue_2))
    (Variables|/Game/Blueprints/GameInstance_Bomb.GameInstance_Bomb_C|SetBox1Size _asgame_instance_bomb "40.000000,300.000000,100.000000")
    (bind _asplayer_1 (Utilities|Casting|CastToPlayer1 OtherActor))
    (Variables|/Game/Blueprints/Player1.Player1_C|SetMaxBombTemp _asplayer_1 (Variables|/Game/Blueprints/Player1.Player1_C|GetMaxBombNumber _asplayer_1))
    (Variables|/Game/Blueprints/Player1.Player1_C|SetBomb _asplayer_1 "/Game/Blueprints/BombRemote.BombRemote_C")
    (Variables|/Game/Blueprints/Player1.Player1_C|SetbHasRemoteBomb _asplayer_1 true)
    (Actor|DestroyActor :!label _label)
    (elif (== _returnvalue "/Game/Blueprints/Player2.Player2_C")
      (bind _asgame_instance_bomb_2 (Utilities|Casting|CastToGameInstance_Bomb _returnvalue_2))
      (Variables|/Game/Blueprints/GameInstance_Bomb.GameInstance_Bomb_C|SetBox2Size _asgame_instance_bomb_2 "40.000000,300.000000,100.000000")
      (bind _asplayer_2 (Utilities|Casting|CastToPlayer2 OtherActor))
      (Variables|/Game/Blueprints/Player2.Player2_C|SetMaxBombTemp _asplayer_2 (Variables|/Game/Blueprints/Player2.Player2_C|GetMaxBombNumber _asplayer_2))
      (Variables|/Game/Blueprints/Player2.Player2_C|SetBomb1 _asplayer_2 "/Game/Blueprints/BombRemote.BombRemote_C")
      (Variables|/Game/Blueprints/Player2.Player2_C|SetbHasRemoteBomb _asplayer_2 true)
      (goto _label))))

(event EventBeginPlay)

(event Collision|EventActorBeginOverlap
  (params (OtherActor :type Actor%20Object%20Reference)))

(event EventTick
  (params (DeltaSeconds :type Float%20%28single-precision%29)))

(fn ConstructionScript)