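; A speed boost pickup that raises the movement speed of whichever player touches it.
; Its Box overlap event checks the actor's exact class for Player1 or Player2, with a duplicate branch for each.
; The matching player gets a fixed MovementSpeed, set outright despite the graph comment describing an increase, plus the HasSpeedUp flag.
; The pickup then destroys itself, with no logic here to end the boost.
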(event OnComponentBeginOverlap(Box)
  (params (OverlappedComponent :type Primitive%20Component%20Object%20Reference) (OtherActor :type Actor%20Object%20Reference) (OtherComp :type Primitive%20Component%20Object%20Reference) (OtherBodyIndex :type Integer) (bFromSweep :type Boolean) (SweepResult :type Hit%20Result%20Structure%20%28by%20ref%29))
  (bind _returnvalue (Utilities|GetClass OtherActor))
  ;[1 1 1] Check Which Player has Overlapped the Pickup, and Increase His Movement Speed by 600.
  (if (== _returnvalue "/Game/Blueprints/Player1.Player1_C")
    (bind _asplayer_1 (Utilities|Casting|CastToPlayer1 OtherActor))
    (Variables|/Game/Blueprints/Player1.Player1_C|SetMovementSpeed _asplayer_1 1.1e+04)
    (Variables|/Game/Blueprints/Player1.Player1_C|SetbHasSpeedUp _asplayer_1 true)
    (Actor|DestroyActor :!label _label)
    (elif (== _returnvalue "/Game/Blueprints/Player2.Player2_C")
      (bind _asplayer_2 (Utilities|Casting|CastToPlayer2 OtherActor))
      (Variables|/Game/Blueprints/Player2.Player2_C|SetMovementSpeed _asplayer_2 1.1e+04)
      (Variables|/Game/Blueprints/Player2.Player2_C|SetbHasSpeedUp _asplayer_2 true)
      (goto _label))))

(event EventBeginPlay)

(event Collision|EventActorBeginOverlap
  (params (OtherActor :type Actor%20Object%20Reference)))

(event EventTick
  (params (DeltaSeconds :type Float%20%28single-precision%29)))

(fn ConstructionScript)