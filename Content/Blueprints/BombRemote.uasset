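; BombRemote is Player 1's remote bomb in a Bomberman-style game, detonated when Explosion() sets IsExploded.
; Tick then runs once, scanning two boxes sized from GameInstance to kill players, break walls and update scores.
; It chain-detonates overlapping bombs, though the Down box's plain Bomb branch is disconnected.
; It spawns the explosion effect, decrements Player1's Bombs count and destroys itself after a delay.
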(event EventBeginPlay
  (bind _asgame_instance_bomb (Utilities|Casting|CastToGameInstance_Bomb (Game|GetGameInstance)))
  (Variables|Default|SetGameInstance _asgame_instance_bomb)
  (Components|Box|SetBoxExtent (Variables|Default|GetRight) (Variables|/Game/Blueprints/GameInstance_Bomb.GameInstance_Bomb_C|GetBox1Size _asgame_instance_bomb) true))

(event EventTick
  (params (DeltaSeconds :type Float%20%28single-precision%29))
  (bind _gameinstance (Variables|Default|GetGameInstance))
  (bind _gameinstance_2 (Variables|Default|GetGameInstance))
  (bind _gameinstance_3 (Variables|Default|GetGameInstance))
  (bind _gameinstance_4 (Variables|Default|GetGameInstance))
  (bind _gameinstance_5 (Variables|Default|GetGameInstance))
  (bind _gameinstance_6 (Variables|Default|GetGameInstance))
  (if (Variables|Default|GetisExploded)
    (Utilities|FlowControl|DoOnce false
      (:Completed
        (Utilities|FlowControl|Sequence
          (:then_0
            (bind _output_get (Variables|Default|SetObjectsOverlapping (Collision|GetOverlappingActors (Variables|Default|GetRight) 0 :!class /Script/Engine.PrimitiveComponent)))
            ;[1 1 1] Check If any player or breakable wall in the explosion area. If so, destroy them all!
            (for _array_element _output_get
              (if (== (Utilities|GetClass _array_element) "/Game/Blueprints/Player1.Player1_C")
                (Variables|/Game/Blueprints/GameInstance_Bomb.GameInstance_Bomb_C|SetP2Score _gameinstance_6 (+ (Variables|/Game/Blueprints/GameInstance_Bomb.GameInstance_Bomb_C|GetP2Score _gameinstance_6) 5e+01))
                (Variables|/Game/Blueprints/GameInstance_Bomb.GameInstance_Bomb_C|SetPlayer1Dead _gameinstance true)
                (Actor|DestroyActor _array_element :!label _label)
                (elif (== (Utilities|GetClass _array_element) "/Game/Blueprints/Player2.Player2_C")
                  (Variables|/Game/Blueprints/GameInstance_Bomb.GameInstance_Bomb_C|SetP1Score _gameinstance_6 (+ (Variables|/Game/Blueprints/GameInstance_Bomb.GameInstance_Bomb_C|GetP1Score _gameinstance_6) 5e+01))
                  (Variables|/Game/Blueprints/GameInstance_Bomb.GameInstance_Bomb_C|SetPlayer2Dead _gameinstance true)
                  (goto _label)
                  (elif (== (Utilities|GetClass _array_element) "/Game/Blueprints/BreakWall.BreakWall_C")
                    (bind _asbreak_wall (Utilities|Casting|CastToBreakWall _array_element))
                    (Variables|/Game/Blueprints/GameInstance_Bomb.GameInstance_Bomb_C|SetP1Score _gameinstance_5 (+ (Variables|/Game/Blueprints/GameInstance_Bomb.GameInstance_Bomb_C|GetP1Score _gameinstance_5) 5.0))
                    (Actor|DestroyActor _asbreak_wall)
                    (elif (== (Utilities|GetClass _array_element) "/Game/Blueprints/Bomb.Bomb_C")
                      (bind _asbomb (Utilities|Casting|CastToBomb _array_element))
                      (Default|Explosion _asbomb)
                      (elif (== (Utilities|GetClass _array_element) "/Game/Blueprints/Bomb1.Bomb1_C")
                        (bind _asbomb_1 (Utilities|Casting|CastToBomb1 _array_element))
                        (Default|Explosion _asbomb_1)
                        (elif (== (Utilities|GetClass _array_element) "BombRemote_C")
                          (bind _asbomb_remote (Utilities|Casting|CastToBombRemote _array_element))
                          (CallFunction|Explosion _asbomb_remote)
                          (elif (== (Utilities|GetClass _array_element) "/Game/Blueprints/BombRemote1.BombRemote1_C")
                            (bind _asbomb_remote_1 (Utilities|Casting|CastToBombRemote1 _array_element))
                            (Default|Explosion _asbomb_remote_1))))))))))
          (:then_1
            (bind _output_get_2 (Variables|Default|SetObjectsOverlapping2 (Collision|GetOverlappingActors (Variables|Default|GetDown) 0 :!class /Script/Engine.PrimitiveComponent)))
            (for _array_element_2 _output_get_2
              (if (== (Utilities|GetClass _array_element_2) "/Game/Blueprints/Player1.Player1_C")
                (Variables|/Game/Blueprints/GameInstance_Bomb.GameInstance_Bomb_C|SetP2Score _gameinstance_3 (+ (Variables|/Game/Blueprints/GameInstance_Bomb.GameInstance_Bomb_C|GetP2Score _gameinstance_3) 5e+01))
                (Variables|/Game/Blueprints/GameInstance_Bomb.GameInstance_Bomb_C|SetPlayer1Dead _gameinstance_4 true)
                (Actor|DestroyActor _array_element_2 :!label _label_2)
                (elif (== (Utilities|GetClass _array_element_2) "/Game/Blueprints/Player2.Player2_C")
                  (Variables|/Game/Blueprints/GameInstance_Bomb.GameInstance_Bomb_C|SetP1Score _gameinstance_3 (+ (Variables|/Game/Blueprints/GameInstance_Bomb.GameInstance_Bomb_C|GetP1Score _gameinstance_3) 5e+01))
                  (Variables|/Game/Blueprints/GameInstance_Bomb.GameInstance_Bomb_C|SetPlayer2Dead _gameinstance_4 true)
                  (goto _label_2)
                  (elif (== (Utilities|GetClass _array_element_2) "/Game/Blueprints/BreakWall.BreakWall_C")
                    (bind _asbreak_wall_2 (Utilities|Casting|CastToBreakWall _array_element_2))
                    (Variables|/Game/Blueprints/GameInstance_Bomb.GameInstance_Bomb_C|SetP1Score _gameinstance_2 (+ (Variables|/Game/Blueprints/GameInstance_Bomb.GameInstance_Bomb_C|GetP1Score _gameinstance_2) 5.0))
                    (Actor|DestroyActor _asbreak_wall_2)
                    (elif (not (== (Utilities|GetClass _array_element_2) "/Game/Blueprints/Bomb.Bomb_C"))
                      (if (== (Utilities|GetClass _array_element_2) "/Game/Blueprints/Bomb1.Bomb1_C")
                        (bind _asbomb_1_2 (Utilities|Casting|CastToBomb1 _array_element_2))
                        (Default|Explosion _asbomb_1_2)
                        (elif (== (Utilities|GetClass _array_element_2) "BombRemote_C")
                          (bind _asbomb_remote_2 (Utilities|Casting|CastToBombRemote _array_element_2))
                          (CallFunction|Explosion _asbomb_remote_2)
                          (elif (== (Utilities|GetClass _array_element_2) "/Game/Blueprints/BombRemote1.BombRemote1_C")
                            (bind _asbomb_remote_1_2 (Utilities|Casting|CastToBombRemote1 _array_element_2))
                            (Default|Explosion _asbomb_remote_1_2)))))))))
            ;[1 1 1] Spawn Particle when Bomb explode
            (Effects|SpawnEmitteratLocation "/Game/StarterContent/Particles/P_Explosion.P_Explosion" (Transformation|GetWorldLocation (Variables|Default|GetSphere)))
            (Components|DestroyComponent (Variables|Default|GetSphere))
            (bind _outactors (Actor|GetAllActorsOfClass "/Game/Blueprints/Player1.Player1_C"))
            (for _array_element_3 _outactors
              (Math|Integer|DecrementInt (Variables|/Game/Blueprints/Player1.Player1_C|GetBombs _array_element_3)
                (:%20%20
                  (Utilities|FlowControl|Delay 1.0)
                  (Actor|DestroyActor))))))))))

(fn ConstructionScript)

(fn Explosion
  (if (not (Variables|Default|GetisExploded))
    (Variables|Default|SetisExploded true)))